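; BP_DoubleBase is a modular room piece, apparently double-width, that assembles its walls in the Construction Script.
; It applies floor, roof and beam materials, then switches on the right, left, back-left and back-right wall settings to add door or solid wall meshes.
; Each wall gets the wall material plus an unlit silhouette second slot, and back doors add an extra mesh.
; It has no active runtime logic.
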(event EventBeginPlay)

(event Collision|EventActorBeginOverlap
  (params (OtherActor :type Actor%20Object%20Reference)))

(event EventTick
  (params (DeltaSeconds :type Float%20%28single-precision%29)))

(fn ConstructionScript
  (Rendering|Material|SetMaterial (Variables|Default|Getgeo_singleRoomLeft_single_floor) 0 (Variables|Materials|GetFloorMaterial))
  (Rendering|Material|SetMaterial (Variables|Default|Getgeo_singleRoomLeft_single_roof) 0 (Variables|Materials|GetFloorMaterial))
  (Rendering|Material|SetMaterial (Variables|Default|Getgeo_singleRoomLeft_single_beams) 0 (Variables|Materials|GetBeamMaterial))
  (Utilities|FlowControl|Sequence
    (:then_0
      (switch Utilities|FlowControl|Switch|SwitchonE_WallChoice (Variables|Default|GetRightWall)
        (:NewEnumerator0
          (bind _returnvalue (AddComponent|AddStaticMeshComponent false))
          (Rendering|Material|SetMaterial _returnvalue 1 "/Game/Environment/Rooms/MAT_unlitSilhouette.MAT_unlitSilhouette")
          (Rendering|Material|SetMaterial _returnvalue 0 (Variables|Materials|GetWallMaterial)))
        (:NewEnumerator1
          (bind _returnvalue_2 (AddComponent|AddStaticMeshComponent false))
          (Rendering|Material|SetMaterial _returnvalue_2 1 "/Game/Environment/Rooms/MAT_unlitSilhouette.MAT_unlitSilhouette")
          (Rendering|Material|SetMaterial _returnvalue_2 0 (Variables|Materials|GetWallMaterial)))))
    (:then_1
      (switch Utilities|FlowControl|Switch|SwitchonE_WallChoice (Variables|Default|GetLeftWall)
        (:NewEnumerator0
          (bind _returnvalue_3 (AddComponent|AddStaticMeshComponent false))
          (Rendering|Material|SetMaterial _returnvalue_3 1 "/Game/Environment/Rooms/MAT_unlitSilhouette.MAT_unlitSilhouette")
          (Rendering|Material|SetMaterial _returnvalue_3 0 (Variables|Materials|GetWallMaterial)))
        (:NewEnumerator1
          (bind _returnvalue_4 (AddComponent|AddStaticMeshComponent false))
          (Rendering|Material|SetMaterial _returnvalue_4 1 "/Game/Environment/Rooms/MAT_unlitSilhouette.MAT_unlitSilhouette")
          (Rendering|Material|SetMaterial _returnvalue_4 0 (Variables|Materials|GetWallMaterial)))))
    (:then_2
      (switch Utilities|FlowControl|Switch|SwitchonE_WallChoice (Variables|Default|GetBackLeftWall)
        (:NewEnumerator0
          (bind _returnvalue_5 (AddComponent|AddStaticMeshComponent false))
          (Rendering|Material|SetMaterial _returnvalue_5 1 "/Game/Environment/Rooms/MAT_unlitSilhouette.MAT_unlitSilhouette")
          (Rendering|Material|SetMaterial _returnvalue_5 0 (Variables|Materials|GetWallMaterial))
          (AddComponent|AddStaticMeshComponent false))
        (:NewEnumerator1
          (bind _returnvalue_6 (AddComponent|AddStaticMeshComponent false))
          (Rendering|Material|SetMaterial _returnvalue_6 1 "/Game/Environment/Rooms/MAT_unlitSilhouette.MAT_unlitSilhouette")
          (Rendering|Material|SetMaterial _returnvalue_6 0 (Variables|Materials|GetWallMaterial)))))
    (:then_3
      (switch Utilities|FlowControl|Switch|SwitchonE_WallChoice (Variables|Default|GetBackRightWall)
        (:NewEnumerator0
          (bind _returnvalue_7 (AddComponent|AddStaticMeshComponent false))
          (Rendering|Material|SetMaterial _returnvalue_7 1 "/Game/Environment/Rooms/MAT_unlitSilhouette.MAT_unlitSilhouette")
          (Rendering|Material|SetMaterial _returnvalue_7 0 (Variables|Materials|GetWallMaterial))
          (AddComponent|AddStaticMeshComponent false))
        (:NewEnumerator1
          (bind _returnvalue_8 (AddComponent|AddStaticMeshComponent false))
          (Rendering|Material|SetMaterial _returnvalue_8 1 "/Game/Environment/Rooms/MAT_unlitSilhouette.MAT_unlitSilhouette")
          (Rendering|Material|SetMaterial _returnvalue_8 0 (Variables|Materials|GetWallMaterial)))))))