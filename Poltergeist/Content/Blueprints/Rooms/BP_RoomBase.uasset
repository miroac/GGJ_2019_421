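; Base room Blueprint that handles camera switching and lets humans claim a room, locking ghosts out.
; On BeginPlay it spawns a room camera, gives child human and ghost interactables a room reference, and prepares the claim material.
; A human entering the transition trigger blends the view to that camera.
; The first object interaction animates the claimed plane's glow and blocks the ghost channel, waiting for an overlap exit if a ghost is inside.
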(event OnComponentBeginOverlap(CameraTransition)
  (params (OverlappedComponent :type Primitive%20Component%20Object%20Reference) (OtherActor :type Actor%20Object%20Reference) (OtherComp :type Primitive%20Component%20Object%20Reference) (OtherBodyIndex :type Integer) (bFromSweep :type Boolean) (SweepResult :type Hit%20Result%20Structure%20%28by%20ref%29))
  (bind _asbp_human (Utilities|Casting|CastToBP_Human OtherActor))
  (bind _asplayer_controller (Utilities|Casting|CastToPlayerController (Pawn|GetController _asbp_human)))
  (Game|Player|SetViewTargetwithBlend _asplayer_controller (Variables|Default|GetRoomCam) (Variables|Default|GetBlendTime) "VTBlend_Linear" 0.0 false))

(event OnComponentBeginOverlap(GhostCollision)
  (params (OverlappedComponent :type Primitive%20Component%20Object%20Reference) (OtherActor :type Actor%20Object%20Reference) (OtherComp :type Primitive%20Component%20Object%20Reference) (OtherBodyIndex :type Integer) (bFromSweep :type Boolean) (SweepResult :type Hit%20Result%20Structure%20%28by%20ref%29))
  (bind _asbp_ghost (Utilities|Casting|CastToBP_Ghost OtherActor)
    (:then
      (Variables|Default|SetGhostInRoomRef _asbp_ghost))
    (:CastFailed
      (bind _asbp_human (Utilities|Casting|CastToBP_Human OtherActor))
      (Variables|Default|SetHumanInRoom _asbp_human))))

(event OnComponentEndOverlap(GhostCollision)
  (params (OverlappedComponent :type Primitive%20Component%20Object%20Reference) (OtherActor :type Actor%20Object%20Reference) (OtherComp :type Primitive%20Component%20Object%20Reference) (OtherBodyIndex :type Integer))
  (if (== OtherActor (Variables|Default|GetHumanInRoom))
    (Variables|Default|SetHumanInRoom 0))
  (Variables|Default|SetGhostInRoomRef 0)
  (if (Variables|Default|GetisRoomHumanControlled)
    (Utilities|FlowControl|DoOnce false
      (:Completed
        (Collision|SetCollisionResponsetoChannel (Variables|Default|GetGhostCollision) "ECC_GameTraceChannel1" "ECR_Block")))))

(event Custom|OnObjectInteracted
  (bind _claimedplanedynamicmat (Variables|Default|GetClaimedPlaneDynamicMat))
  (if (not (Variables|Default|GetisRoomHumanControlled))
    (Variables|Default|SetisRoomHumanControlled true)
    (Utilities|FlowControl|Sequence
      (:then_0
        (Utilities|FlowControl|DoOnce false
          (:Completed
            (bind _materiallerp (Timeline|RoomClaimedLerp PlayFromStart)
              (:Update
                (Rendering|Material|SetScalarParameterValue _claimedplanedynamicmat "emissive" _materiallerp :!class /Script/Engine.MaterialInstanceDynamic))
              (:Finished
                (Rendering|Material|SetScalarParameterValue _claimedplanedynamicmat "emissive" 1e+01 :!class /Script/Engine.MaterialInstanceDynamic))))))
      (:then_1
        (Variables|Default|GetGhostInRoomRef
          (:then)
          (:else
            (Utilities|FlowControl|DoOnce false
              (:Completed
                (Collision|SetCollisionResponsetoChannel (Variables|Default|GetGhostCollision) "ECC_GameTraceChannel1" "ECR_Block")))))))))

(event EventBeginPlay
  (bind _returnvalue (Game|SpawnActorfromClass "/Script/Engine.CameraActor" (Transformation|GetWorldTransform (Variables|Default|GetCamera)) "AlwaysSpawn" 0 0))
  (Variables|Default|SetRoomCam _returnvalue)
  (Utilities|FlowControl|Sequence
    (:then_0
      (Utilities|Array|Clear (Variables|Default|GetHumanInteractives))
      (for _array_element (Actor|GetAllChildActors true)
        (bind _asbp_human_interactable (Utilities|Casting|CastToBP_HumanInteractable _array_element))
        (Utilities|Array|AddUnique (Variables|Default|GetHumanInteractives) _asbp_human_interactable)
        (Variables|/Game/Blueprints/BP_Interactable.BP_Interactable_C|SetRoomRef _asbp_human_interactable self)))
    (:then_1
      (Utilities|Array|Clear (Variables|Default|GetGhostInteractives))
      (for _array_element_2 (Actor|GetAllChildActors true)
        (bind _asbp_ghost_interactable (Utilities|Casting|CastToBP_GhostInteractable _array_element_2))
        (Utilities|Array|AddUnique (Variables|Default|GetHumanInteractives) 0)
        (Variables|/Game/Blueprints/BP_Interactable.BP_Interactable_C|SetRoomRef _asbp_ghost_interactable self)))
    (:then_2
      (bind _returnvalue_2 (Rendering|Material|CreateDynamicMaterialInstance (Variables|Default|GetClaimedPlane) 0 "/Game/Effects/GlowyThing/MAT_CLAIMED.MAT_CLAIMED" "None" :!class /Script/Engine.PrimitiveComponent))
      (bind _output_get (Variables|Default|SetClaimedPlaneDynamicMat _returnvalue_2))
      (Rendering|Material|SetScalarParameterValue _output_get "emissive" 0.0 :!class /Script/Engine.MaterialInstanceDynamic))))

(fn ConstructionScript)