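; BP_Elevator is an elevator that carries a BP_Human between a lower and an upper trigger box, in either direction.
; Overlapping either box stores the start and end transforms, disables the human's movement and mesh collision, then plays a timeline that lerps the actor across.
; On finish it restores walking and collision, with an IsTeleporting flag blocking new overlaps during the trip.
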(event OnComponentBeginOverlap(LowerBox)
  (params (OverlappedComponent :type Primitive%20Component%20Object%20Reference) (OtherActor :type Actor%20Object%20Reference) (OtherComp :type Primitive%20Component%20Object%20Reference) (OtherBodyIndex :type Integer) (bFromSweep :type Boolean) (SweepResult :type Hit%20Result%20Structure%20%28by%20ref%29))
  (if (not (Variables|Default|GetbIsTeleporting))
    (Variables|Default|SetHumanActorRef OtherActor)
    (Variables|Default|SetStartTransform (Transformation|GetWorldTransform (Variables|Default|GetLowerBox)))
    (Variables|Default|SetEndTransform (Transformation|GetWorldTransform (Variables|Default|GetUpperBox)))
    (bind _asbp_human (Utilities|Casting|CastToBP_Human (Variables|Default|GetHumanActorRef)))
    (Pawn|Components|CharacterMovement|DisableMovement (Variables|/Script/Engine.Character|GetCharacterMovement _asbp_human))
    (Collision|SetCollisionEnabled (Variables|/Script/Engine.Character|GetMesh _asbp_human) "NoCollision")
    (Variables|Default|SetbIsTeleporting true)
    (bind _lerppos (Timeline|HumanMoveTimeline PlayFromStart)
      (:Update
        (Transformation|SetActorTransform (Variables|Default|GetHumanActorRef) (Math|Transform|Lerp(Transform) (Variables|Default|GetStartTransform) (Variables|Default|GetEndTransform) _lerppos)))
      (:Finished
        (Transformation|SetActorTransform (Variables|Default|GetHumanActorRef) (Variables|Default|GetEndTransform))
        (bind _asbp_human_2 (Utilities|Casting|CastToBP_Human (Variables|Default|GetHumanActorRef)))
        (Pawn|Components|CharacterMovement|SetMovementMode (Variables|/Script/Engine.Character|GetCharacterMovement _asbp_human_2) "MOVE_Walking" 0)
        (Collision|SetCollisionEnabled (Variables|/Script/Engine.Character|GetMesh _asbp_human_2) "QueryAndPhysics")
        (Variables|Default|SetHumanActorRef 0)
        (Variables|Default|SetbIsTeleporting false)))))

(event OnComponentBeginOverlap(UpperBox)
  (params (OverlappedComponent :type Primitive%20Component%20Object%20Reference) (OtherActor :type Actor%20Object%20Reference) (OtherComp :type Primitive%20Component%20Object%20Reference) (OtherBodyIndex :type Integer) (bFromSweep :type Boolean) (SweepResult :type Hit%20Result%20Structure%20%28by%20ref%29))
  (if (not (Variables|Default|GetbIsTeleporting))
    (Variables|Default|SetHumanActorRef OtherActor)
    (Variables|Default|SetStartTransform (Transformation|GetWorldTransform (Variables|Default|GetUpperBox)))
    (Variables|Default|SetEndTransform (Transformation|GetWorldTransform (Variables|Default|GetLowerBox)))
    (bind _asbp_human (Utilities|Casting|CastToBP_Human (Variables|Default|GetHumanActorRef)))
    (Pawn|Components|CharacterMovement|DisableMovement (Variables|/Script/Engine.Character|GetCharacterMovement _asbp_human))
    (Collision|SetCollisionEnabled (Variables|/Script/Engine.Character|GetMesh _asbp_human) "NoCollision")
    (Variables|Default|SetbIsTeleporting true)
    (bind _lerppos (Timeline|HumanMoveTimeline PlayFromStart)
      (:Update
        (Transformation|SetActorTransform (Variables|Default|GetHumanActorRef) (Math|Transform|Lerp(Transform) (Variables|Default|GetStartTransform) (Variables|Default|GetEndTransform) _lerppos)))
      (:Finished
        (Transformation|SetActorTransform (Variables|Default|GetHumanActorRef) (Variables|Default|GetEndTransform))
        (bind _asbp_human_2 (Utilities|Casting|CastToBP_Human (Variables|Default|GetHumanActorRef)))
        (Pawn|Components|CharacterMovement|SetMovementMode (Variables|/Script/Engine.Character|GetCharacterMovement _asbp_human_2) "MOVE_Walking" 0)
        (Collision|SetCollisionEnabled (Variables|/Script/Engine.Character|GetMesh _asbp_human_2) "QueryAndPhysics")
        (Variables|Default|SetHumanActorRef 0)
        (Variables|Default|SetbIsTeleporting false)))))

(fn ConstructionScript)