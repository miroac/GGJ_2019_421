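; Game mode for a multiplayer match with one ghost and two humans.
; BeginPlay caches spawn transforms from tagged actors in the level.
; PostLogin collects joining controllers and, once the third is added at index 2, shuffles the list to randomize roles and starts the game.
; BeginGame spawns BP_Ghost or BP_Human by array index and possesses it; the third human spawn and SpawnGhostPawn helper are unused here.
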(event Custom|BeginGame
  (for (_array_element _array_index) (Variables|Default|GetListOfPlayers)
    (switch int _array_index
      (:0
        (bind _asbp_game_pc (Utilities|Casting|CastToBP_Game_PC _array_element))
        (bind _returnvalue (Game|SpawnActorfromClass "/Game/Blueprints/BP_Ghost.BP_Ghost_C" (Variables|SpawnPositions|GetGhostStartLoc) "Undefined" 0 0))
        (Pawn|Possess _asbp_game_pc _returnvalue))
      (:1
        (bind _asbp_game_pc_2 (Utilities|Casting|CastToBP_Game_PC _array_element))
        (bind _returnvalue_2 (Game|SpawnActorfromClass "/Game/Blueprints/BP_Human.BP_Human_C" (Variables|SpawnPositions|GetPlayer1StartLoc) "Undefined" 0 0))
        (Pawn|Possess _asbp_game_pc_2 _returnvalue_2))
      (:2
        (bind _asbp_game_pc_3 (Utilities|Casting|CastToBP_Game_PC _array_element))
        (bind _returnvalue_3 (Game|SpawnActorfromClass "/Game/Blueprints/BP_Human.BP_Human_C" (Variables|SpawnPositions|GetPlayer2StartLoc) "Undefined" 0 0))
        (Pawn|Possess _asbp_game_pc_3 _returnvalue_3)))))

(event EventBeginPlay
  (bind _returnvalue (CallFunction|GetPlayerStartPos "GhostSpawn"))
  (Variables|SpawnPositions|SetGhostStartLoc _returnvalue)
  (bind _returnvalue_2 (CallFunction|GetPlayerStartPos "Player1Spawn"))
  (Variables|SpawnPositions|SetPlayer1StartLoc _returnvalue_2)
  (bind _returnvalue_3 (CallFunction|GetPlayerStartPos "Player2Spawn"))
  (Variables|SpawnPositions|SetPlayer2StartLoc _returnvalue_3)
  (bind _returnvalue_4 (CallFunction|GetPlayerStartPos "Player3Spawn"))
  (Variables|SpawnPositions|SetPlayer3StartLoc _returnvalue_4))

(event EventPostLogin
  (params (NewPlayer :type Player%20Controller%20Object%20Reference))
  (bind _returnvalue (Utilities|Array|Add (Variables|Default|GetListOfPlayers) NewPlayer))
  (if (== _returnvalue 2)
    (Utilities|Array|Shuffle (Variables|Default|GetListOfPlayers))
    (CallFunction|BeginGame)))

(fn ConstructionScript)

(fn SpawnGhostPawn
  (params (SpawnTransform :type Transform) (PlayerController :type Player%20Controller%20Object%20Reference))
  (bind _returnvalue (Game|SpawnActorfromClass "/Game/Blueprints/BP_Ghost.BP_Ghost_C" SpawnTransform "Undefined" 0 0))
  (Pawn|Possess PlayerController _returnvalue))

(fn GetPlayerStartPos
  (params (Tag :type Name))
  (bind _outactors (Actor|GetAllActorswithTag Tag))
  (Utilities|IsValid (Utilities|Array|Get(acopy) _outactors)
    (:Is%20Valid
      (return (Transformation|GetActorTransform (Utilities|Array|Get(acopy) _outactors))))))