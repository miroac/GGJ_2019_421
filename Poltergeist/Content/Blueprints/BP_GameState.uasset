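; BP_GameState tracks the round clock and ends the match as a loss for the humans when time runs out.
; On the authority, BeginPlay copies RoundLength from BP_GameMode and binds its game start and end events to set state flags.
; While the game runs, Tick accumulates RoundTimer, prints it as debug text, and on expiry sets HumansWin false and calls EndGame on the game mode.
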(event Custom|HandleOnGameStart
  (Variables|Default|SetgameStarted? true))

(event Custom|HandleOnGameEnd
  (Variables|Default|SetgameEnded? true))

(event EventBeginPlay
  (Networking|SwitchHasAuthority
    (:Authority
      (bind _asbp_game_mode (Utilities|Casting|CastToBP_GameMode (Game|GetGameMode)))
      (Variables|Default|SetRoundLength (Variables|/Game/Blueprints/BP_GameMode.BP_GameMode_C|GetRoundLength _asbp_game_mode))
      (EventDispatchers|BindEventtoOnGameStart _asbp_game_mode (delegate Custom|HandleOnGameStart))
      (EventDispatchers|BindEventtoOnGameEnd _asbp_game_mode (delegate Custom|HandleOnGameEnd)))))

(event EventTick
  (params (DeltaSeconds :type Float%20%28single-precision%29))
  (bind _roundlength (Variables|Default|GetRoundLength))
  (if (and (Variables|Default|GetgameStarted?) (not (Variables|Default|GetgameEnded?)))
    (Variables|Default|SetRoundTimer (+ (Variables|Default|GetRoundTimer) DeltaSeconds))
    (Development|PrintString (Utilities|String|Append "Game Time: " (Utilities|String|ToString(Float) (Variables|Default|GetRoundTimer)) " / " (Utilities|String|ToString(Float) _roundlength)) true true "(R=0.000000,G=0.660000,B=1.000000,A=1.000000)" 0.0001)
    (if (>= (Variables|Default|GetRoundTimer) _roundlength)
      (bind _asbp_game_mode (Utilities|Casting|CastToBP_GameMode (Game|GetGameMode)))
      (Variables|/Game/Blueprints/BP_GameMode.BP_GameMode_C|SetbHumansWin _asbp_game_mode false)
      (Default|EndGame _asbp_game_mode))))

(fn ConstructionScript)