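; Game mode for an asymmetric human-versus-ghost match that adds a local player on BeginPlay.
; A DoOnce-guarded setup, called from both BeginPlay and PostLogin, caches the human and ghost start actors.
; PostLogin collects controllers and starts the game when their count reaches the target.
; StartGame spawns a human for the first controller and a ghost for the second at random matching starts, then possesses them.
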(event Custom|StartGame
  (bind _playercontrollers (Variables|Default|GetPlayerControllers))
  (bind _humanplayerstarts (Variables|Default|GetHumanPlayerStarts))
  (bind _ghostplayerstarts (Variables|Default|GetGhostPlayerStarts))
  (bind _output (Utilities|Array|Get(acopy) _playercontrollers 1))
  (bind _output_2 (Utilities|Array|Get(acopy) _playercontrollers))
  (Utilities|FlowControl|Sequence
    (:then_0
      (bind _returnvalue (Game|SpawnActorfromClass "/Game/Blueprints/BP_Human.BP_Human_C" (Transformation|GetActorTransform (Utilities|Array|Get(acopy) _humanplayerstarts (Math|Random|RandomIntegerinRange 0 (- (Utilities|Array|Length _humanplayerstarts) 1)))) "AdjustIfPossibleButAlwaysSpawn" _output_2 0))
      (Utilities|IsValid _returnvalue
        (:Is%20Valid
          (Pawn|Possess _output_2 _returnvalue))))
    (:then_1
      (bind _returnvalue_2 (Game|SpawnActorfromClass "/Game/Blueprints/BP_Ghost.BP_Ghost_C" (Transformation|GetActorTransform (Utilities|Array|Get(acopy) _ghostplayerstarts (Math|Random|RandomIntegerinRange 0 (- (Utilities|Array|Length _ghostplayerstarts) 1)))) "AdjustIfPossibleButAlwaysSpawn" _output 0))
      (Utilities|IsValid _returnvalue_2
        (:Is%20Valid
          (Pawn|Possess _output _returnvalue_2))))))

(event Custom|SetupPlayerStarts
  (Utilities|FlowControl|DoOnce false
    (:Completed
      (bind _outactors (Actor|GetAllActorsOfClass "/Game/Blueprints/BP_HumanStart.BP_HumanStart_C"))
      (Variables|Default|SetHumanPlayerStarts _outactors)
      (bind _outactors_2 (Actor|GetAllActorsOfClass "/Game/Blueprints/BP_GhostStart.BP_GhostStart_C"))
      (Variables|Default|SetGhostPlayerStarts _outactors_2))))

(event EventBeginPlay
  (CallFunction|SetupPlayerStarts)
  (Class|GameplayStatics|CreatePlayer -1))

(event EventPostLogin
  (params (NewPlayer :type Player%20Controller%20Object%20Reference))
  (bind _playercontrollers (Variables|Default|GetPlayerControllers))
  (CallFunction|SetupPlayerStarts)
  (Utilities|Array|AddUnique _playercontrollers NewPlayer)
  ;[1 1 1] two players joined, ready to start
  (if (== (Utilities|Array|Length _playercontrollers) (Variables|Default|GetTargetPlayerCount))
    (CallFunction|StartGame)))

(fn ConstructionScript)