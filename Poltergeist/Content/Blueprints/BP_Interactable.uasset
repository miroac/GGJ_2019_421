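; BP_Interactable is an actor that humans, ghosts or both can interact with, as set by per-type flags.
; A Box overlap records an eligible BP_Human or BP_Ghost as CurrentCollidingActor and shows the InteractBillboard prompt until that actor leaves.
; Start, cancel and finish events track IsInteracting with placeholder debug prints.
; Finishing also disables further interaction and hides the prompt.
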(event OnComponentBeginOverlap(Box)
  (params (OverlappedComponent :type Primitive%20Component%20Object%20Reference) (OtherActor :type Actor%20Object%20Reference) (OtherComp :type Primitive%20Component%20Object%20Reference) (OtherBodyIndex :type Integer) (bFromSweep :type Boolean) (SweepResult :type Hit%20Result%20Structure%20%28by%20ref%29))
  (if (and (or (and (Variables|Default|GetbInteractableByHuman) (.bSuccess (Utilities|Casting|CastToBP_Human OtherActor))) (and (Variables|Default|GetbInteractableByGhost) (.bSuccess (Utilities|Casting|CastToBP_Ghost OtherActor)))) (Variables|Default|GetbIsInteractable))
    (Variables|Default|SetCurrentCollidingActor OtherActor)
    (Development|SetHiddeninGame (Variables|Default|GetInteractBillboard) false false)))

(event OnComponentEndOverlap(Box)
  (params (OverlappedComponent :type Primitive%20Component%20Object%20Reference) (OtherActor :type Actor%20Object%20Reference) (OtherComp :type Primitive%20Component%20Object%20Reference) (OtherBodyIndex :type Integer))
  (if (== OtherActor (Variables|Default|GetCurrentCollidingActor))
    (Variables|Default|SetCurrentCollidingActor 0)
    (Development|SetHiddeninGame (Variables|Default|GetInteractBillboard) true false)))

(event Custom|OnFinishInteracting
  (Development|PrintString "DO OBJECT INTERACTION HERE")
  (Variables|Default|SetbIsInteractable false)
  (Development|SetHiddeninGame (Variables|Default|GetInteractBillboard) true false)
  (Variables|Default|SetIsInteracting false))

(event Custom|OnStartInteracting
  (Development|PrintString "OBJECT START INTERACTION HERE")
  (Variables|Default|SetIsInteracting true))

(event Custom|OnCancelInteracting
  (Development|PrintString "PREMATURE END!!!")
  (Variables|Default|SetIsInteracting false))

(event EventBeginPlay)

(event Collision|EventActorBeginOverlap
  (params (OtherActor :type Actor%20Object%20Reference)))

(event EventTick
  (params (DeltaSeconds :type Float%20%28single-precision%29)))

(fn ConstructionScript)