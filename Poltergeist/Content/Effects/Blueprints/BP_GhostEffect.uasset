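; BP_GhostEffect is a ghost visual effect actor that combines a Niagara system with a point light and reacts to its parent actor's movement.
; Each tick, the parent's normalized speed samples a color curve for both particle and light color and scales the particle spawn rate.
; TriggerPull feeds a target position, scaled pull strength and on/off interaction scale into the Niagara user parameters.
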(event Custom|TriggerPull
  (params (TargetPosition :type Vector) (TargetScale :type Float%20%28single-precision%29) (IsInteracting :type Boolean))
  (bind _niagara (Variables|Default|GetNiagara))
  (bind _niagara_2 (Variables|Default|GetNiagara))
  (Class|NiagaraComponent|SetNiagaraVariableVec3 _niagara "User.Target" TargetPosition)
  (Niagara|SetNiagaraVariable(Float) _niagara "User.TargetStrength" (* TargetScale (Variables|Default|GetPullStrength)))
  (if IsInteracting
    (Niagara|SetNiagaraVariable(Float) _niagara_2 "User.InteractScale" 1.0)
    (else
      (Niagara|SetNiagaraVariable(Float) _niagara_2 "User.InteractScale" 0.0))))

(event EventTick
  (params (DeltaSeconds :type Float%20%28single-precision%29))
  (bind _returnvalue (Actor|GetParentActor))
  (bind _colorcurve (Variables|Default|GetColorCurve))
  (bind _returnvalue_2 (Transformation|GetVelocity _returnvalue))
  (bind _returnvalue_3 (Math|Vector|VectorLength _returnvalue_2))
  (bind _returnvalue_4 (/ _returnvalue_3 6e+02))
  (bind _returnvalue_5 (Math|Curves|GetLinearColorValue _colorcurve _returnvalue_4))
  (Niagara|SetNiagaraVariable(LinearColor) (Variables|Default|GetNiagara) "User.ParticleColor" _returnvalue_5)
  (Rendering|Components|Light|SetLightColor (Variables|Default|GetPointLight) _returnvalue_5 true)
  (Niagara|SetNiagaraVariable(Float) (Variables|Default|GetNiagara) "User.SpawnRate" (Math|Float|Lerp 5e+01 3e+02 _returnvalue_4)))

(fn ConstructionScript)